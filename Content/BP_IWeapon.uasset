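; BP_IWeapon is a Blueprint interface, judging by its name and stub functions, for querying and changing weapon status.
; It declares getter and setter pairs for an enum weapon state, an enum combat value and a boolean move permission.
; It also declares a current-weapon query and a weapon-change call.
; All functions are empty or return defaults, leaving the behavior to implementers.
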(fn `GetWeapon_Combat`
  (returns (Combat :type "/Game/Enum/E_CombatMode Enum"))
  (return "NewEnumerator0"))

(fn `GetWeapon_Current`)

(fn `GetWeapon_Move`
  (returns (CanMove :type Boolean))
  (return false))

(fn `GetWeapon_State`
  (returns (State :type "/Game/Enum/E_PlayerState Enum"))
  (return "NewEnumerator0"))

(fn `SetWeapon_Combat`
  (params (Combat :type "/Game/Enum/E_CombatMode Enum" :default "NewEnumerator0"))
  (returns (Result :type "/Game/Enum/E_CombatMode Enum"))
  (return "NewEnumerator0"))

(fn `SetWeapon_Move`
  (params (CanMove :type Boolean))
  (returns (Result :type Boolean))
  (return false))

(fn `SetWeapon_State`
  (params (State :type "/Game/Enum/E_PlayerState Enum" :default "NewEnumerator0"))
  (returns (Result :type "/Game/Enum/E_PlayerState Enum"))
  (return "NewEnumerator0"))

(fn `Weapon_Change`)