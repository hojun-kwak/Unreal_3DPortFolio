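; BP_Items is an item actor for weapons, apparently a base class given its empty Attack and EndAttack stubs.
; Tick shows ItemComent and turns it toward the player within 300 units horizontally, hiding it otherwise.
; Weapon state, combat, movement, type and ID pass to the owner through BP_IItems, and CanAttack compares combat type and state.
; SendDamage ignores the owner, disables the hit Box and applies Power damage to Characters.
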(event `self.ReceiveBeginPlay`)

(event `self.ReceiveTick`
  (params (DeltaSeconds :type "Float (single-precision)"))
  (bind _itemcoment (`self.ItemComent`))
  (if (< (`KismetMathLibrary.VSizeXY` (- (`self.K2_GetActorLocation` (`GameplayStatics.GetPlayerPawn` 0)) (`self.K2_GetActorLocation` (`ActorComponent.GetOwner` (`self.ItemComent`))))) 300.0)
    (`SceneComponent.SetVisibility` _itemcoment true false)
    (`SceneComponent.K2_SetWorldRotation` (`self.ItemComent`) (`KismetMathLibrary.FindLookAtRotation` (`self.K2_GetActorLocation` (`ActorComponent.GetOwner` (`self.ItemComent`))) (`self.K2_GetActorLocation` (`GameplayStatics.GetPlayerPawn` 0))) false false)
    (else
      (`SceneComponent.SetVisibility` _itemcoment false false))))

(fn `Attack`)

(fn `CanAttack`
  (returns (ReturnValue :type Boolean))
  (return (== (`|EnumEquality` (`self.CombatType`) (`self.GetWeapon_Combat`)) (`|EnumEquality` (`self.GetWeapon_State`) "NewEnumerator0"))))

(fn `Does_Interface`
  (returns (ReturnValue :type Boolean))
  (return (`KismetSystemLibrary.DoesImplementInterface` (`self.GetOwner`) "/Game/BP_IItems.BP_IItems_C")))

(fn `EndAttack`)

(fn `GetMove`
  (returns (CanMove :type Boolean))
  (if (`self.Does_Interface`)
    (bind _canmove (message `/Game/BP_IItems.GetWeapon_Move` (`self.GetOwner`)))
    (return _canmove)))

(fn `GetWeapon_Combat`
  (returns (Combat :type "/Game/Enum/E_CombatMode Enum"))
  (if (`self.Does_Interface`)
    (bind _combat (message `/Game/BP_IItems.GetWeapon_Combat` (`self.GetOwner`)))
    (return _combat)))

(fn `GetWeapon_ID`
  (returns (WeaponID :type Integer))
  (if (`self.Does_Interface`)
    (bind _weaponid (message `/Game/BP_IItems.GetWeapon_ID` (`self.GetOwner`)))
    (return _weaponid)))

(fn `GetWeapon_State`
  (returns (State :type "/Game/Enum/E_PlayerState Enum"))
  (if (`self.Does_Interface`)
    (bind _state (message `/Game/BP_IItems.GetWeapon_State` (`self.GetOwner`)))
    (return _state)))

(fn `GetWeapon_Type`
  (returns (Type :type "/Game/안지워지는쓰레기/E_WeaponType Enum"))
  (if (`self.Does_Interface`)
    (bind _weapontype (message `/Game/BP_IItems.GetWeapon_Type` (`self.GetOwner`)))
    (return _weapontype)))

(fn `SendDamage`
  (params (OtherActor :type "Actor Object Reference"))
  (returns (Result :type Boolean))
  (if (!= OtherActor (`self.GetOwner`))
    (`PrimitiveComponent.SetCollisionEnabled` (`self.Box`) "NoCollision")
    (bind _ascharacter (cast `Character` OtherActor))
    (`GameplayStatics.ApplyDamage` _ascharacter (`self.Power`) (`self.GetInstigatorController` (`self.GetOwner`)) self)
    (return true)
    (else
      (return false))))

(fn `SetMove`
  (params (CanMove :type Boolean))
  (if (`self.Does_Interface`)
    (message `/Game/BP_IItems.SetWeapon_Move` (`self.GetOwner`) CanMove)))

(fn `SetWeapon_Combat`
  (params (Combat :type "/Game/Enum/E_CombatMode Enum" :default "NewEnumerator0"))
  (if (`self.Does_Interface`)
    (message `/Game/BP_IItems.SetWeapon_Combat` (`self.GetOwner`) Combat)))

(fn `SetWeapon_ID`
  (params (WeaponID :type Integer))
  (locals (NewLocalVar_0 :type Boolean :default false))
  (if (`self.Does_Interface`)
    (message `/Game/BP_IItems.SetWeapon_ID` (`self.GetOwner`) WeaponID)))

(fn `SetWeapon_State`
  (params (State :type "/Game/Enum/E_PlayerState Enum" :default "NewEnumerator0"))
  (if (`self.Does_Interface`)
    (message `/Game/BP_IItems.SetWeapon_State` (`self.GetOwner`) State)))

(fn `SetWeapon_Type`
  (params (Type :type "/Game/안지워지는쓰레기/E_WeaponType Enum" :default "NewEnumerator2"))
  (if (`self.Does_Interface`)
    (message `/Game/BP_IItems.SetWeapon_Type` (`self.GetOwner`) Type)))

(fn `UserConstructionScript`)