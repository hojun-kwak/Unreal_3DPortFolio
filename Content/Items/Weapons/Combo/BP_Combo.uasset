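; Combo weapon actor that plays chained melee attack montages on its owning Character for sword and dual-sword combat.
; BeginPlay loads two data tables into per-style arrays, whose rows set montage, play rate, start section and movement permission.
; Attack either starts a combo or, while EnableNextCombo is set, advances the count and buffers the next hit.
; PlayNext events play buffered hits and flag the last step; EndAttack resets everything.
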(event `self.ReceiveBeginPlay`
  (bind _combotables (`self.ComboTables`))
  (bind _output (`|GetArrayItem` _combotables))
  (bind _output_2 (`|GetArrayItem` _combotables 1))
  ;[1 1 1] ComboTable Ready
  (`|ExecutionSequence`
    (:`then_0`
      (bind _outrownames (`DataTableFunctionLibrary.GetDataTableRowNames` _output))
      (for _array_element _outrownames
        (bind _returnvalue (`|GetDataTableRow` _output _array_element)
          (:`then`
            (`KismetArrayLibrary.Array_Add` (`self.SwordCombo`) _returnvalue)))))
    (:`then_1`
      (bind _outrownames_2 (`DataTableFunctionLibrary.GetDataTableRowNames` _output_2))
      (for _array_element_2 _outrownames_2
        (bind _returnvalue_2 (`|GetDataTableRow` _output_2 _array_element_2)
          (:`then`
            (`KismetArrayLibrary.Array_Add` (`self.DualSwordCombo`) _returnvalue_2)))))))

(event `self.Attack`
  ;[1 1 1] Attack
  (if (`self.EnableNextCombo`)
    (`/Engine/EditorBlueprintResources/StandardMacros.IncrementInt` (`self.ComboCount`)
      (:`  `
        (set `self.ExistNextCombo` true)
        (set `self.EnableNextCombo` false)))
    (elif (`self.CanAttack`)
      (switch `/Game/Enum/E_CombatMode` (`self.CombatType`)
        (:`NewEnumerator2`
          (`self.SetWeapon_State` "NewEnumerator2")
          (`self.PlayComboMontage`))
        (:`NewEnumerator3`
          (`self.SetWeapon_State` "NewEnumerator2")
          (`self.PlayComboDual`))))))

(event `PlayNextCombo`
  ;[1 1 1] NextCombo
  (if (`self.ExistNextCombo`)
    (`self.PlayComboMontage`)
    (set `self.ExistNextCombo` false)
    (set `self.LastCombo` (== (- (`KismetArrayLibrary.Array_Length` (`self.SwordCombo`)) 1) (`self.ComboCount`)))))

(event `PlayNextDualCombo`
  ;[1 1 1] NextDualCombo
  (if (`self.ExistNextCombo`)
    (`self.PlayComboDual`)
    (set `self.ExistNextCombo` false)
    (set `self.LastCombo` (== (- (`KismetArrayLibrary.Array_Length` (`self.DualSwordCombo`)) 1) (`self.ComboCount`)))))

(event `self.EndAttack`
  ;[1 1 1] EndAttack
  (`self.SetWeapon_State` "NewEnumerator0")
  (`self.SetMove` true)
  (set `self.ComboCount` 0)
  (set `self.ExistNextCombo` false)
  (set `self.LastCombo` true))

(fn `PlayComboDual`
  (bind (_output_montage _output_playrate _output_stratsectionname _output_canmove) (break `/Game/DataTable/FCombo_Table` (`|GetArrayItem` (`self.DualSwordCombo`) (`self.ComboCount`))))
  (bind _ascharacter (cast `Character` (`self.GetOwner`)))
  (`Character.PlayAnimMontage` _ascharacter _output_montage _output_playrate _output_stratsectionname)
  (`self.SetMove` _output_canmove))

(fn `PlayComboMontage`
  (bind (_output_montage _output_playrate _output_stratsectionname _output_canmove) (break `/Game/DataTable/FCombo_Table` (`|GetArrayItem` (`self.SwordCombo`) (`self.ComboCount`))))
  (bind _ascharacter (cast `Character` (`self.GetOwner`)))
  (`Character.PlayAnimMontage` _ascharacter _output_montage _output_playrate _output_stratsectionname)
  (`self.SetMove` _output_canmove))

(fn `UserConstructionScript`
  (`parent.UserConstructionScript`))