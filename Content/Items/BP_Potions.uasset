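; BP_Potions is a potion item actor that sets its appearance from a data table according to its PotionID.
; On BeginPlay, a nonzero ID becomes the row name for a PotionData_Table lookup, whose mesh is applied to the skeletal mesh with a fixed rotation.
; Parent BeginPlay runs only when that row is found.
; Tick and construction only call the parent, and the overlap event is empty.
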(event `self.ReceiveBeginPlay`
  (bind _skeletalmesh (`self.SkeletalMesh`))
  (if (!= (`self.Potion_ID`) 0)
    (bind _returnvalue (`|GetDataTableRow` "/Game/DataTable/PotionData_Table.PotionData_Table" (`KismetStringLibrary.Conv_StringToName` (`KismetStringLibrary.Conv_IntToString` (`self.Potion_ID`))))
      (:`then`
        (`SkinnedMeshComponent.SetSkinnedAssetAndUpdate` _skeletalmesh (`.Mesh_17_2AAF91724D4BF81069BCACBA9B6C402D` (break `/Game/DataTable/FPotion_Table` _returnvalue)) true)
        (`SceneComponent.K2_SetRelativeRotation` _skeletalmesh (struct :`Roll` 90.0) false false)
        (`parent.ReceiveBeginPlay`)))))

(event `self.ReceiveTick`
  (params (DeltaSeconds :type "Float (single-precision)"))
  (`parent.ReceiveTick` DeltaSeconds))

(fn `UserConstructionScript`
  (`parent.UserConstructionScript`))