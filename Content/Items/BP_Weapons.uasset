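; BP_Weapons is a weapon item Blueprint that takes its appearance from a data table.
; On BeginPlay, a nonzero WeaponID is converted to a row name and looked up in WeaponData_Table, then the row's mesh is applied to the SkeletalMesh with a fixed relative rotation.
; Parent BeginPlay runs only when that row is found, while Tick and the construction script just call the parent.
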(event `self.ReceiveBeginPlay`
  (bind _skeletalmesh (`self.SkeletalMesh`))
  (if (!= (`self.WeaponID`) 0)
    (bind _returnvalue (`|GetDataTableRow` "/Game/DataTable/WeaponData_Table.WeaponData_Table" (`KismetStringLibrary.Conv_StringToName` (`KismetStringLibrary.Conv_IntToString` (`self.WeaponID`))))
      (:`then`
        (`SkinnedMeshComponent.SetSkinnedAssetAndUpdate` _skeletalmesh (`.Mesh_17_2AAF91724D4BF81069BCACBA9B6C402D` (break `/Game/DataTable/FWeapon_Table` _returnvalue)) true)
        (`SceneComponent.K2_SetRelativeRotation` _skeletalmesh (struct :`Roll` 90.0) false false)
        (`parent.ReceiveBeginPlay`)))))

(event `self.ReceiveTick`
  (params (DeltaSeconds :type "Float (single-precision)"))
  (`parent.ReceiveTick` DeltaSeconds))

(fn `UserConstructionScript`
  (`parent.UserConstructionScript`))