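; BP_FieldItem is a field item actor that spawns a data-driven weapon and shows a widget when the player is near.
; On BeginPlay, a non-zero ItemClassId selects an ItemData_Table row, and that row's Weapon class is spawned at the row's Location with a fixed rotation.
; Each Tick, it shows the widget and turns it toward the player pawn within a short horizontal distance, otherwise hiding it.
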(event `self.ReceiveBeginPlay`
  (if (!= (`self.ItemClassId`) 0)
    (bind _returnvalue (`|GetDataTableRow` "/Game/DataTable/ItemData_Table.ItemData_Table" (`KismetStringLibrary.Conv_StringToName` (`KismetStringLibrary.Conv_IntToString` (`self.ItemClassId`))))
      (:`then`
        (bind (_itemid _itemname _mesh _staticmesh _weapon _location) (break `/Game/DataTable/FItem_Table` _returnvalue))
        (`|SpawnActorFromClass` _weapon (`KismetMathLibrary.MakeTransform` _location (struct :`Roll` 90.0)) "Undefined" "OverrideRootScale" null null)))))

(event `self.ReceiveTick`
  (params (DeltaSeconds :type "Float (single-precision)"))
  (bind _widget_0 (`self.Widget_0`))
  (if (< (`KismetMathLibrary.VSizeXY` (- (`self.K2_GetActorLocation` (`GameplayStatics.GetPlayerPawn` 0)) (`self.K2_GetActorLocation` (`ActorComponent.GetOwner` (`self.SkeletalMesh_0`))))) 300.0)
    (`SceneComponent.SetVisibility` _widget_0 true false)
    (`SceneComponent.K2_SetWorldRotation` (`self.Widget_0`) (`KismetMathLibrary.FindLookAtRotation` (`self.K2_GetActorLocation` (`ActorComponent.GetOwner` (`self.SkeletalMesh_0`))) (`self.K2_GetActorLocation` (`GameplayStatics.GetPlayerPawn` 0))) false false)
    (else
      (`SceneComponent.SetVisibility` _widget_0 false false))))

(fn `UserConstructionScript`)