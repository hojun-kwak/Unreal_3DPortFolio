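; Weapon actor, apparently a base class with empty Attack and EndAttack stubs, that loads its skeletal mesh from a data table by WeaponID.
; Tick shows an item component facing the player when nearby in XY.
; Combat, state, type and movement are read and written on the owner through BP_IWeapon, with the first two feeding CanAttack.
; SendDamage applies Power damage to Characters other than the owner.
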(event `self.ReceiveBeginPlay`
  (bind _skeletalmesh (`self.SkeletalMesh`))
  (if (!= (`self.WeaponID`) 0)
    (bind _returnvalue (`|GetDataTableRow` "/Game/DataTable/WeaponData_Table.WeaponData_Table" (`KismetStringLibrary.Conv_StringToName` (`KismetStringLibrary.Conv_IntToString` (`self.WeaponID`))))
      (:`then`
        (`SkinnedMeshComponent.SetSkinnedAssetAndUpdate` _skeletalmesh (`.Mesh_55_D33520D54B940B31CE74FDAE60749397` (break `/Game/DataTable/FItem_Table` _returnvalue)) true)
        (`SceneComponent.K2_SetRelativeRotation` _skeletalmesh (struct :`Roll` 90.0) false false)))))

(event `self.ReceiveTick`
  (params (DeltaSeconds :type "Float (single-precision)"))
  (bind _itemcoment (`self.ItemComent`))
  (if (< (`KismetMathLibrary.VSizeXY` (- (`self.K2_GetActorLocation` (`GameplayStatics.GetPlayerPawn` 0)) (`self.K2_GetActorLocation` (`ActorComponent.GetOwner` (`self.ItemComent`))))) 300.0)
    (`SceneComponent.SetVisibility` _itemcoment true false)
    (`SceneComponent.K2_SetWorldRotation` (`self.ItemComent`) (`KismetMathLibrary.FindLookAtRotation` (`self.K2_GetActorLocation` (`ActorComponent.GetOwner` (`self.ItemComent`))) (`self.K2_GetActorLocation` (`GameplayStatics.GetPlayerPawn` 0))) false false)
    (else
      (`SceneComponent.SetVisibility` _itemcoment false false))))

(fn `Attack`)

(fn `CanAttack`
  (returns (ReturnValue :type Boolean))
  (return (== (`|EnumEquality` (`self.CombatType`) (`self.GetWeapon_Combat`)) (`|EnumEquality` (`self.GetWeapon_State`) "NewEnumerator0"))))

(fn `Does_Interface`
  (returns (ReturnValue :type Boolean))
  (return (`KismetSystemLibrary.DoesImplementInterface` (`self.GetOwner`) "/Game/BP_IWeapon.BP_IWeapon_C")))

(fn `EndAttack`)

(fn `GetMove`
  (returns (CanMove :type Boolean))
  (if (`self.Does_Interface`)
    (bind _canmove (message `/Game/BP_IWeapon.GetWeapon_Move` (`self.GetOwner`)))
    (return _canmove)))

(fn `GetWeapon_Combat`
  (returns (Combat :type "/Game/Enum/E_CombatMode Enum"))
  (if (`self.Does_Interface`)
    (bind _combat (message `/Game/BP_IWeapon.GetWeapon_Combat` (`self.GetOwner`)))
    (return _combat)))

(fn `GetWeapon_State`
  (returns (State :type "/Game/Enum/E_PlayerState Enum"))
  (if (`self.Does_Interface`)
    (bind _state (message `/Game/BP_IWeapon.GetWeapon_State` (`self.GetOwner`)))
    (return _state)))

(fn `GetWeapon_Type`
  (returns (Type :type "/Game/Enum/E_WeaponType Enum"))
  (if (`self.Does_Interface`)
    (bind _weapontype (message `/Game/BP_IWeapon.GetWeapon_Type` (`self.GetOwner`)))
    (return _weapontype)))

(fn `SendDamage`
  (params (OtherActor :type "Actor Object Reference"))
  (if (!= OtherActor (`self.GetOwner`))
    (bind _ascharacter (cast `Character` OtherActor))
    (`GameplayStatics.ApplyDamage` _ascharacter (`self.Power`) (`self.GetInstigatorController` (`self.GetOwner`)) self)))

(fn `SetMove`
  (params (CanMove :type Boolean))
  (if (`self.Does_Interface`)
    (message `/Game/BP_IWeapon.SetWeapon_Move` (`self.GetOwner`) CanMove)))

(fn `SetWeapon_Combat`
  (params (Combat :type "/Game/Enum/E_CombatMode Enum" :default "NewEnumerator0"))
  (if (`self.Does_Interface`)
    (message `/Game/BP_IWeapon.SetWeapon_Combat` (`self.GetOwner`) Combat)))

(fn `SetWeapon_State`
  (params (State :type "/Game/Enum/E_PlayerState Enum" :default "NewEnumerator0"))
  (if (`self.Does_Interface`)
    (message `/Game/BP_IWeapon.SetWeapon_State` (`self.GetOwner`) State)))

(fn `SetWeapon_Type`
  (params (Type :type "/Game/Enum/E_WeaponType Enum" :default "NewEnumerator2"))
  (if (`self.Does_Interface`)
    (message `/Game/BP_IWeapon.SetWeapon_Type` (`self.GetOwner`) Type)))

(fn `UserConstructionScript`)