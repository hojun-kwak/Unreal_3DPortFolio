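; BP_Combo is a weapon Blueprint that plays multi-step attack combos on its owning Character.
; BeginPlay caches montage entries from a data table, each setting play rate, start section and whether movement is allowed.
; Attack starts the first montage, or queues the next step while the combo window is open.
; PlayNextCombo plays any queued step and flags the last one, while EndAttack resets weapon state, movement and combo tracking.
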(event `self.ReceiveBeginPlay`
  ;[1 1 1] BeginPlay
  (bind _outrownames (`DataTableFunctionLibrary.GetDataTableRowNames` (`self.ComboTable`)))
  (for _array_element _outrownames
    (bind _returnvalue (`|GetDataTableRow` (`self.ComboTable`) _array_element)
      (:`then`
        (`KismetArrayLibrary.Array_Add` (`self.ComboMontage`) _returnvalue)))))

(event `self.Attack`
  ;[1 1 1] Attack
  (if (`self.EnableNextCombo`)
    (`/Engine/EditorBlueprintResources/StandardMacros.IncrementInt` (`self.ComboCount`)
      (:`  `
        (set `self.ExistNextCombo` true)
        (set `self.EnableNextCombo` false)))
    (elif (`self.CanAttack`)
      (`self.SetWeapon_State` "NewEnumerator2")
      (`self.PlayComboMontage`))))

(event `PlayNextCombo`
  ;[1 1 1] NextCombo
  (if (`self.ExistNextCombo`)
    (`self.PlayComboMontage`)
    (set `self.ExistNextCombo` false)
    (set `self.LastCombo` (== (- (`KismetArrayLibrary.Array_Length` (`self.ComboMontage`)) 1) (`self.ComboCount`)))))

(event `self.EndAttack`
  ;[1 1 1] EndAttack
  (`self.SetWeapon_State` "NewEnumerator0")
  (`self.SetMove` true)
  (set `self.ComboCount` 0)
  (set `self.ExistNextCombo` false)
  (set `self.LastCombo` true))

(fn `PlayComboMontage`
  (bind (_output_montage _output_playrate _output_stratsectionname _output_canmove) (break `/Game/DataTable/FCombo_Table` (`|GetArrayItem` (`self.ComboMontage`) (`self.ComboCount`))))
  (bind _ascharacter (cast `Character` (`self.GetOwner`)))
  (`Character.PlayAnimMontage` _ascharacter _output_montage _output_playrate _output_stratsectionname)
  (`self.SetMove` _output_canmove))

(fn `UserConstructionScript`
  (`parent.UserConstructionScript`))