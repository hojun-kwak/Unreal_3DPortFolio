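; BP_Sword2 is a sword weapon actor that shows a widget when the player pawn is nearby.
; Every Tick it measures the horizontal distance from the skeletal mesh's owner to player pawn 0 and toggles the widget's visibility against a fixed radius.
; While visible, the widget turns to face the player, using a look-at rotation from the actor's location to the pawn's.
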(event `self.ReceiveTick`
  (params (DeltaSeconds :type "Float (single-precision)"))
  (bind _widget (`self.Widget`))
  (if (< (`KismetMathLibrary.VSizeXY` (- (`self.K2_GetActorLocation` (`GameplayStatics.GetPlayerPawn` 0)) (`self.K2_GetActorLocation` (`ActorComponent.GetOwner` (`self.SkeletalMesh`))))) 300.0)
    (`SceneComponent.SetVisibility` _widget true false)
    (`SceneComponent.K2_SetWorldRotation` (`self.Widget`) (`KismetMathLibrary.FindLookAtRotation` (`self.K2_GetActorLocation` (`ActorComponent.GetOwner` (`self.SkeletalMesh`))) (`self.K2_GetActorLocation` (`GameplayStatics.GetPlayerPawn` 0))) false false)
    (else
      (`SceneComponent.SetVisibility` _widget false false))))

(fn `UserConstructionScript`)