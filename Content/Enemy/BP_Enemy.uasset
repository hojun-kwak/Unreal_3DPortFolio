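; Enemy character that takes damage, shows a health bar widget and dies when HP runs out.
; AnyDamage lowers HP, snaps the enemy toward its attacker, then either plays a hit reaction with mass-scaled knockback or a death montage before destroying it.
; Tick shows the bar only while LookAtPlayer is set.
; Weapon interface functions are stubs; distance-based visibility and older Hit/Die logic are unwired.
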(event `self.ReceiveBeginPlay`
  (`|ExecutionSequence`
    (:`then_0`
      (`self.UpdateHpBar`))
    (:`then_1`
      (`self.OnSetVisivility`))
    (:`then_2`
      (set `self.State` "NewEnumerator1"))))

(event `self.ReceiveAnyDamage`
  (params (Damage :type "Float (single-precision)") (DamageType :type "DamageType Object Reference") (InstigatedBy :type "Controller Object Reference") (DamageCauser :type "Actor Object Reference"))
  (bind _ascharacter (cast `Character` (`Controller.K2_GetPawn` InstigatedBy)))
  (set `self.Attacker` _ascharacter)
  (set `self.Damage` Damage)
  (set `self.NowHp` (- (`self.NowHp`) (`self.Damage`)))
  (`self.UpdateHpBar`)
  (`self.K2_SetActorRotation` (`KismetMathLibrary.FindLookAtRotation` (`self.K2_GetActorLocation`) (`self.K2_GetActorLocation` (`self.Attacker`))))
  (if (<= (`self.NowHp`) 0.0)
    (`/Engine/EditorBlueprintResources/StandardMacros.DoOnce` false
      (:`Completed`
        (set `self.State` "NewEnumerator4")
        (`PrimitiveComponent.SetCollisionEnabled` (`self.CapsuleComponent`) "NoCollision")
        (bind _returnvalue (`self.PlayAnimMontage` "/Game/Character/Mongtagu/GetHitBackFall_Montage.GetHitBackFall_Montage" 1.0 "Start"))
        (`KismetSystemLibrary.Delay` (- _returnvalue 1.5))
        (`self.K2_DestroyActor`)))
    (else
      (`self.PlayAnimMontage` "/Game/Character/Mongtagu/Hit_Reaction_Montage.Hit_Reaction_Montage" 3.0)
      (`self.K2_AddActorWorldOffset` (* (`KismetMathLibrary.Vector_Normal2D` (`self.GetActorForwardVector`)) (* (`CharacterMovementComponent.Mass` (`self.CharacterMovement`)) -0.2))))))

(event `Player Distance To Enemy`
  (if (<= (`self.GetDistanceTo` (`GameplayStatics.GetPlayerCharacter` 0) self) 500.0)
    (`self.OnSetVisivility`)
    (else
      (`self.OffSetVisivility`))))

(event `self.ReceiveTick`
  (params (DeltaSeconds :type "Float (single-precision)"))
  (bind _hpbar (`self.Hpbar`))
  (`|ExecutionSequence`
    (:`then_0`
      (if (`self.LookAtPlayer`)
        (`SceneComponent.SetHiddenInGame` _hpbar false false)
        (else
          (`SceneComponent.SetHiddenInGame` _hpbar true false))))))

(fn `GetWeapon_Combat`
  (returns (Combat :type "/Game/Enum/E_CombatMode Enum"))
  (return "NewEnumerator0"))

(fn `GetWeapon_Current`
  (returns (Weapon :type "/Game/Items/BP_Items Object Reference"))
  (return null))

(fn `GetWeapon_ID`
  (returns (WeaponID :type Integer))
  (return 0))

(fn `GetWeapon_Move`
  (returns (CanMove :type Boolean))
  (return false))

(fn `GetWeapon_State`
  (returns (State :type "/Game/Enum/E_PlayerState Enum"))
  (return "NewEnumerator0"))

(fn `GetWeapon_Type`
  (returns (WeaponType :type "/Game/안지워지는쓰레기/E_WeaponType Enum"))
  (return "NewEnumerator2"))

(fn `OffSetVisivility`
  (`SceneComponent.SetVisibility` (`self.Mesh`) false false)
  (`SceneComponent.SetVisibility` (`self.Hpbar`) false false)
  (`SceneComponent.SetVisibility` (`self.ParticleSystem`) true false))

(fn `OnSetVisivility`
  (`SceneComponent.SetVisibility` (`self.Mesh`) true false)
  (`SceneComponent.SetVisibility` (`self.Hpbar`) true false)
  (`SceneComponent.SetVisibility` (`self.ParticleSystem`) false false))

(fn `SetWeapon_Combat`
  (params (Combat :type "/Game/Enum/E_CombatMode Enum" :default "NewEnumerator0"))
  (returns (Result :type "/Game/Enum/E_CombatMode Enum"))
  (return "NewEnumerator0"))

(fn `SetWeapon_ID`
  (params (WeaponID :type Integer))
  (returns (Result :type Integer))
  (return 0))

(fn `SetWeapon_Move`
  (params (CanMove :type Boolean))
  (returns (Result :type Boolean))
  (return false))

(fn `SetWeapon_State`
  (params (State :type "/Game/Enum/E_PlayerState Enum" :default "NewEnumerator0"))
  (returns (Result :type "/Game/Enum/E_PlayerState Enum"))
  (return "NewEnumerator0"))

(fn `SetWeapon_Type`
  (params (WeaponType :type "/Game/안지워지는쓰레기/E_WeaponType Enum" :default "NewEnumerator2"))
  (returns (Result :type "/Game/안지워지는쓰레기/E_WeaponType Enum"))
  (return "NewEnumerator2"))

(fn `UpdateHpBar`
  (bind _aswg_hp_bar (cast `/Game/Widget/WG_HpBar` (`WidgetComponent.GetUserWidgetObject` (`self.Hpbar`))))
  (`/Game/Widget/WG_HpBar.UpdataHpBar` _aswg_hp_bar (`self.NowHp`)))

(fn `UserConstructionScript`)

(fn `Weapon_Change`
  (params (`New Weapon` :type "/Game/Items/BP_Items Object Reference"))
  (returns (Weapon :type "/Game/Items/BP_Items Object Reference"))
  (return null))