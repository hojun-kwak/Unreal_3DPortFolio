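; AI controller for the random-type enemy, running its behavior tree and seeding Direction and IsAlive on the blackboard.
; Tick sets FindPlayer from a signed X-offset check, true unless the player is over 300 units toward negative X.
; Tick and successful perception share a branch setting CanSeePlayer when FindPlayer holds and the perceived actor is BP_Player.
; Failed perception clears CanSeePlayer.
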(event `self.ReceiveBeginPlay`
  (`self.RunBehaviorTree` "/Game/Enemy/AI/Enemy_Type/Random_AI/BT_AI_Random_Enemy.BT_AI_Random_Enemy")
  (bind _asbp_ai_random_enemy (cast `/Game/Enemy/AI/Enemy_Type/Random_AI/BP_AI_Random_Enemy` (`self.K2_GetPawn` self)))
  (set `self.AI` _asbp_ai_random_enemy)
  (`BlackboardComponent.SetValueAsInt` (`AIBlueprintHelperLibrary.GetBlackboard` null) "Direction" 1)
  (`BlackboardComponent.SetValueAsBool` (`AIBlueprintHelperLibrary.GetBlackboard` null) "IsAlive" true))

(event `self.ReceivePossess`
  (params (PossessedPawn :type "Pawn Object Reference")))

(event `self.ReceiveTick`
  (params (DeltaSeconds :type "Float (single-precision)"))
  (bind _returnvalue_x (`KismetMathLibrary.BreakVector` (`self.K2_GetActorLocation` (`self.AI`))))
  (bind _returnvalue_x_2 (`KismetMathLibrary.BreakVector` (`self.K2_GetActorLocation` (`GameplayStatics.GetPlayerPawn` 0))))
  (`|ExecutionSequence`
    (:`then_0`
      (if (>= (- _returnvalue_x_2 _returnvalue_x) -300.0)
        (set `self.FindPlayer` true)
        (else
          (set `self.FindPlayer` false)))
      (if (`self.FindPlayer`) :!label _label
        (cast `/Game/Player/BP_Player` (stale `self.AIPerception.OnTargetPerceptionUpdated` Actor))
        (`BlackboardComponent.SetValueAsBool` (`AIBlueprintHelperLibrary.GetBlackboard` null) "CanSeePlayer" true)))))

(event `self.AIPerception.OnTargetPerceptionUpdated`
  (params (Actor :type "Actor Object Reference") (Stimulus :type "AIStimulus Structure"))
  (if (`.bSuccessfullySensed` (break `AIStimulus` Stimulus))
    (goto _label)
    (else
      (`BlackboardComponent.SetValueAsBool` (`AIBlueprintHelperLibrary.GetBlackboard` null) "CanSeePlayer" false))))

(fn `UserConstructionScript`)