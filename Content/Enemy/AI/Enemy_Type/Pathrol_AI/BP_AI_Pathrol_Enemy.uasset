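; Patrol-type enemy character that builds on a parent enemy Blueprint, adding player awareness and randomized melee attacks.
; Each tick it copies FindPlayer from its BP_AI_Controller_Pathroll into LookAtPlayer, then runs the parent tick, which is skipped if that controller cast fails.
; The Melee event plays one of three attack montages at random on the mesh.
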(event `self.ReceiveBeginPlay`
  (`parent.ReceiveBeginPlay`))

(event `self.ReceiveTick`
  (params (DeltaSeconds :type "Float (single-precision)"))
  (`|ExecutionSequence`
    (:`then_0`
      (bind _asbp_ai_controller_pathroll (cast `/Game/Enemy/AI/Enemy_Type/Pathrol_AI/BP_AI_Controller_Pathroll` (`AIBlueprintHelperLibrary.GetAIController` self)))
      (set `self.LookAtPlayer` (`/Game/Enemy/AI/Enemy_Type/Pathrol_AI/BP_AI_Controller_Pathroll.FindPlayer` _asbp_ai_controller_pathroll))
      (`parent.ReceiveTick` DeltaSeconds))))

(event `self.Melee`
  (bind _mesh (`self.Mesh`))
  (switch `int` (`KismetMathLibrary.RandomInteger` 3)
    (:`0`
      (`|PlayMontage` _mesh "/Game/Character/Mongtagu/Enemy/Enemy_Attack.Enemy_Attack"))
    (:`1`
      (`|PlayMontage` _mesh "/Game/Character/Mongtagu/Enemy/Enemy_Attack2.Enemy_Attack2"))
    (:`2`
      (`|PlayMontage` _mesh "/Game/Character/Mongtagu/Enemy/Enemy_Attack3.Enemy_Attack3"))))

(fn `UserConstructionScript`
  (`parent.UserConstructionScript`))