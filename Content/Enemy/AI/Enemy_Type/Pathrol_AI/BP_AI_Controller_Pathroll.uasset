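; AI controller for the patrol enemy, running its patrol behavior tree and feeding it blackboard data.
; On possession it copies looping and wait time from the pawn's patrol path and sets an initial direction.
; Tick switches the pawn's state and a FindPlayer flag using a signed X-offset threshold to the player.
; AI Perception updates CanSeePlayer, with successful sightings gated by that flag and a player cast.
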(event `self.ReceivePossess`
  (params (PossessedPawn :type "Pawn Object Reference"))
  (`self.RunBehaviorTree` "/Game/Enemy/AI/Enemy_Type/Pathrol_AI/BT_AI_Pathrol_Enemy.BT_AI_Pathrol_Enemy")
  (bind _asbp_ai_pathrol_enemy (cast `/Game/Enemy/AI/Enemy_Type/Pathrol_AI/BP_AI_Pathrol_Enemy` (`self.K2_GetPawn` self)))
  (bind _output_get (set `self.MyPawn` _asbp_ai_pathrol_enemy))
  (bind _pathrolpaths (`/Game/Enemy/AI/Enemy_Type/Pathrol_AI/BP_AI_Pathrol_Enemy.PathrolPaths` _output_get))
  (`/Engine/EditorBlueprintResources/StandardMacros.IsValid` _pathrolpaths
    (:`Is Valid`
      (`BlackboardComponent.SetValueAsBool` (`AIBlueprintHelperLibrary.GetBlackboard` null) "PathLooping" (`/Game/Enemy/AI/BP_PathrollPath.IsLooping` _pathrolpaths))
      (`BlackboardComponent.SetValueAsFloat` (`AIBlueprintHelperLibrary.GetBlackboard` null) "WaitTime" (`/Game/Enemy/AI/BP_PathrollPath.WaitTime` (`/Game/Enemy/AI/Enemy_Type/Pathrol_AI/BP_AI_Pathrol_Enemy.PathrolPaths` (`self.MyPawn`)))))
    (:`Is Not Valid`
      _))
  (`BlackboardComponent.SetValueAsInt` (`AIBlueprintHelperLibrary.GetBlackboard` null) "Direction" 1))

(event `self.ReceiveTick`
  (params (DeltaSeconds :type "Float (single-precision)"))
  (bind _mypawn (`self.MyPawn`))
  (bind _returnvalue_x (`KismetMathLibrary.BreakVector` (`self.K2_GetActorLocation` (`self.MyPawn`))))
  (bind _returnvalue_x_2 (`KismetMathLibrary.BreakVector` (`self.K2_GetActorLocation` (`GameplayStatics.GetPlayerPawn` 0))))
  (if (>= (- _returnvalue_x_2 _returnvalue_x) -600.0)
    (set `/Game/Enemy/BP_Enemy.State` "NewEnumerator2" _mypawn)
    (set `self.FindPlayer` true)
    (else
      (set `/Game/Enemy/BP_Enemy.State` "NewEnumerator1" _mypawn)
      (set `self.FindPlayer` false)))
  (if (`self.FindPlayer`) :!label _label
    (cast `/Game/Player/BP_Player` (stale `self.AIPerception.OnTargetPerceptionUpdated` Actor))
    (`BlackboardComponent.SetValueAsBool` (`AIBlueprintHelperLibrary.GetBlackboard` null) "CanSeePlayer" (`.bSuccessfullySensed` (break `AIStimulus` (stale `self.AIPerception.OnTargetPerceptionUpdated` Stimulus))))))

(event `self.AIPerception.OnTargetPerceptionUpdated`
  (params (Actor :type "Actor Object Reference") (Stimulus :type "AIStimulus Structure"))
  (bind (_age _expirationage _strength _stimuluslocation _receiverlocation _tag _bsuccessfullysensed) (break `AIStimulus` Stimulus))
  (if _bsuccessfullysensed
    (goto _label)
    (else
      (`BlackboardComponent.SetValueAsBool` (`AIBlueprintHelperLibrary.GetBlackboard` null) "CanSeePlayer" _bsuccessfullysensed))))

(fn `UserConstructionScript`)