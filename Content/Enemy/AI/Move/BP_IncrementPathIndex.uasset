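; Behavior tree task that advances an enemy's patrol path index in the forward direction.
; When the Blackboard direction is forward, it checks the next index against the path array on the controlled BP_AI_Pathrol_Enemy.
; It stores the incremented index and succeeds, or at the last point flips the direction to backward and fails.
; It also fails when the direction is not forward.
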(event `self.ReceiveExecuteAI`
  (params (OwnerController :type "AIController Object Reference") (ControlledPawn :type "Pawn Object Reference"))
  (bind _bb_direction (`self.BB_Direction`))
  (bind _returnvalue (+ (`BTFunctionLibrary.GetBlackboardValueAsInt` (`self.BB_PathIndex`)) 1))
  (if (== (`BTFunctionLibrary.GetBlackboardValueAsInt` (`self.BB_Direction`)) 1)
    (bind _asbp_ai_pathrol_enemy (cast `/Game/Enemy/AI/Enemy_Type/Pathrol_AI/BP_AI_Pathrol_Enemy` ControlledPawn))
    (if (<= _returnvalue (- (`KismetArrayLibrary.Array_Length` (`/Game/Enemy/AI/BP_PathrollPath.PathrollPaths` (`/Game/Enemy/AI/Enemy_Type/Pathrol_AI/BP_AI_Pathrol_Enemy.PathrolPaths` _asbp_ai_pathrol_enemy))) 1))
      (`BTFunctionLibrary.SetBlackboardValueAsInt` _bb_direction 1)
      (`BTFunctionLibrary.SetBlackboardValueAsInt` (`self.BB_PathIndex`) _returnvalue)
      (`self.FinishExecute` true)
      (else
        (`BTFunctionLibrary.SetBlackboardValueAsInt` _bb_direction -1)
        (`self.FinishExecute` false)))
    (else
      (`self.FinishExecute` false))))