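; Behavior tree task that gives a patrolling enemy AI its next move target from its assigned patrol path.
; It reads the point at the blackboard's path index, converts it from the path actor's local space to world space and stores it as the path vector.
; It then writes the configured state to both the blackboard and the pawn, finishing successfully; an invalid path leaves the task unfinished.
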(event `self.ReceiveExecuteAI`
  (params (OwnerController :type "AIController Object Reference") (ControlledPawn :type "Pawn Object Reference"))
  (bind _state (`self.State`))
  (bind _asbp_ai_pathrol_enemy (cast `/Game/Enemy/AI/Enemy_Type/Pathrol_AI/BP_AI_Pathrol_Enemy` ControlledPawn))
  (bind _pathrolpaths (`/Game/Enemy/AI/Enemy_Type/Pathrol_AI/BP_AI_Pathrol_Enemy.PathrolPaths` _asbp_ai_pathrol_enemy)
    (:`then`
      (`BTFunctionLibrary.SetBlackboardValueAsVector` (`self.BB_PathVector`) (`KismetMathLibrary.TransformLocation` (`Actor.GetTransform` _pathrolpaths) (`|GetArrayItem` (`/Game/Enemy/AI/BP_PathrollPath.PathrollPaths` _pathrolpaths) (`BTFunctionLibrary.GetBlackboardValueAsInt` (`self.BB_PathIndex`)))))
      (`BTFunctionLibrary.SetBlackboardValueAsEnum` (`self.BB_State`) _state)
      (bind _asbp_ai (cast `/Game/Enemy/AI/BP_AI` ControlledPawn))
      (set `/Game/Enemy/BP_Enemy.State` _state _asbp_ai)
      (`self.FinishExecute` true))
    (:`else`)))