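; Boss enemy Blueprint that controls when the player's boss HP bar is on screen.
; BeginPlay runs the parent logic, then calls OnSetVisivility.
; Tick checks distance to player 0 every frame and shows BP_Player's BossHpBar within 600 units, otherwise hides it.
; Unconnected leftover nodes for visibility calls, an actor move and a jump montage never run.
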(event `self.ReceiveBeginPlay`
  (`parent.ReceiveBeginPlay`)
  (`|ExecutionSequence`
    (:`then_0`
      (`self.OnSetVisivility`))))

(event `self.ReceiveTick`
  (params (DeltaSeconds :type "Float (single-precision)"))
  (`parent.ReceiveTick` DeltaSeconds)
  (if (<= (`self.GetDistanceTo` self (`GameplayStatics.GetPlayerCharacter` 0)) 600.0)
    (bind _asbp_player (cast `/Game/Player/BP_Player` (`GameplayStatics.GetPlayerCharacter` 0)))
    (`Widget.SetVisibility` (`/Game/Player/BP_Player.Boss_HpBar` _asbp_player) "Visible")
    (else
      (bind _asbp_player_2 (cast `/Game/Player/BP_Player` (`GameplayStatics.GetPlayerCharacter` 0)))
      (`Widget.SetVisibility` (`/Game/Player/BP_Player.Boss_HpBar` _asbp_player_2) "Hidden"))))

(fn `UserConstructionScript`
  (`parent.UserConstructionScript`))