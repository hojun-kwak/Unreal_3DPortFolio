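; AI controller for BP_AI_Random_Enemy that runs BT_AI_Random_Enemy on possession and seeds its Direction blackboard key to 1.
; Each tick, the player's X offset from the enemy against a -600 threshold sets the enemy State and FindPlayer flag.
; AI perception updates write CanSeePlayer, with successful sightings requiring FindPlayer and a BP_Player target.
; Tick also feeds that same gated write, reusing the perception event's outputs.
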(event `self.ReceivePossess`
  (params (PossessedPawn :type "Pawn Object Reference"))
  (`self.RunBehaviorTree` "/Game/Enemy/AI/Enemy_Type/Random_AI/BT_AI_Random_Enemy.BT_AI_Random_Enemy")
  (bind _asbp_ai_random_enemy (cast `/Game/Enemy/AI/Enemy_Type/Random_AI/BP_AI_Random_Enemy` (`self.K2_GetPawn` self)))
  (set `self.AI` _asbp_ai_random_enemy)
  (`BlackboardComponent.SetValueAsInt` (`AIBlueprintHelperLibrary.GetBlackboard` null) "Direction" 1))

(event `self.ReceiveTick`
  (params (DeltaSeconds :type "Float (single-precision)"))
  (bind _ai (`self.AI`))
  (bind _returnvalue_x (`KismetMathLibrary.BreakVector` (`self.K2_GetActorLocation` (`self.AI`))))
  (bind _returnvalue_x_2 (`KismetMathLibrary.BreakVector` (`self.K2_GetActorLocation` (`GameplayStatics.GetPlayerPawn` 0))))
  (if (>= (- _returnvalue_x_2 _returnvalue_x) -600.0)
    (set `/Game/Enemy/BP_Enemy.State` "NewEnumerator2" _ai)
    (set `self.FindPlayer` true)
    (else
      (set `/Game/Enemy/BP_Enemy.State` "NewEnumerator1" _ai)
      (set `self.FindPlayer` false)))
  (if (`self.FindPlayer`) :!label _label
    (cast `/Game/Player/BP_Player` (stale `self.AIPerception.OnTargetPerceptionUpdated` Actor))
    (`BlackboardComponent.SetValueAsBool` (`AIBlueprintHelperLibrary.GetBlackboard` null) "CanSeePlayer" (`.bSuccessfullySensed` (break `AIStimulus` (stale `self.AIPerception.OnTargetPerceptionUpdated` Stimulus))))))

(event `self.AIPerception.OnTargetPerceptionUpdated`
  (params (Actor :type "Actor Object Reference") (Stimulus :type "AIStimulus Structure"))
  (bind (_age _expirationage _strength _stimuluslocation _receiverlocation _tag _bsuccessfullysensed) (break `AIStimulus` Stimulus))
  (if _bsuccessfullysensed
    (goto _label)
    (else
      (`BlackboardComponent.SetValueAsBool` (`AIBlueprintHelperLibrary.GetBlackboard` null) "CanSeePlayer" _bsuccessfullysensed))))

(fn `UserConstructionScript`)