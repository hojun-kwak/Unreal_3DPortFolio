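; AI controller for BP_AI enemies that runs their behavior tree and reports player detection to it.
; On possess, it stores the BP_AI pawn and runs the behavior tree assigned on that pawn.
; Target perception updates involving BP_Player write the sensed result to the CanSeePlayer blackboard bool.
; An unconnected sight-scan branch for setting or clearing a Player blackboard object never runs.
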(event `self.ReceivePossess`
  (params (PossessedPawn :type "Pawn Object Reference"))
  (bind _asbp_ai (cast `/Game/Enemy/BP_AI` PossessedPawn))
  (bind _output_get (set `self.AICharater` _asbp_ai))
  (bind _behaviertree (`/Game/Enemy/BP_AI.BehavierTree` _output_get)
    (:`then`
      (`self.RunBehaviorTree` _behaviertree))
    (:`else`)))

(event `self.AIPerception.OnPerceptionUpdated`
  (params (UpdatedActors :type "Array of Actor Object Reference (by ref)")))

(event `PerceivedBreak`
  (for _array_element (`AIPerceptionComponent.GetCurrentlyPerceivedActors` (`self.AIPerception`) "/Script/AIModule.AISense_Sight") :!via `Break`
    (bind _asbp_player (cast `/Game/Player/BP_Player` _array_element))
    (`BlackboardComponent.SetValueAsObject` (`AIBlueprintHelperLibrary.GetBlackboard` null) "Player" _asbp_player)
    (set `self.FindPlayer` true)
    (`self.PerceivedBreak`))
  (if (not (`self.FindPlayer`))
    (`BlackboardComponent.SetValueAsObject` (`AIBlueprintHelperLibrary.GetBlackboard` null) "Player" null)))

(event `self.AIPerception.OnTargetPerceptionUpdated`
  (params (Actor :type "Actor Object Reference") (Stimulus :type "AIStimulus Structure"))
  (cast `/Game/Player/BP_Player` Actor)
  (`BlackboardComponent.SetValueAsBool` (`AIBlueprintHelperLibrary.GetBlackboard` null) "CanSeePlayer" (`.bSuccessfullySensed` (break `AIStimulus` Stimulus))))

(fn `UserConstructionScript`)