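; BP_IItems is a Blueprint interface, judging by its name and stub functions, that defines a common contract for weapon items.
; It declares getter and setter pairs for weapon state, combat, movement permission, type and ID, plus functions to get the current weapon and change to a new one.
; The functions hold no logic and return only default values, leaving behavior to implementers.
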(fn `GetWeapon_Combat`
  (returns (Combat :type "/Game/Enum/E_CombatMode Enum"))
  (return "NewEnumerator0"))

(fn `GetWeapon_Current`
  (returns (Weapon :type "/Game/Items/BP_Items Object Reference"))
  (return null))

(fn `GetWeapon_ID`
  (returns (WeaponID :type Integer))
  (return 0))

(fn `GetWeapon_Move`
  (returns (CanMove :type Boolean))
  (return false))

(fn `GetWeapon_State`
  (returns (State :type "/Game/Enum/E_PlayerState Enum"))
  (return "NewEnumerator0"))

(fn `GetWeapon_Type`
  (returns (WeaponType :type "/Game/안지워지는쓰레기/E_WeaponType Enum"))
  (return "NewEnumerator2"))

(fn `SetWeapon_Combat`
  (params (Combat :type "/Game/Enum/E_CombatMode Enum" :default "NewEnumerator0"))
  (returns (Result :type "/Game/Enum/E_CombatMode Enum"))
  (return "NewEnumerator0"))

(fn `SetWeapon_ID`
  (params (WeaponID :type Integer))
  (returns (Result :type Integer))
  (return 0))

(fn `SetWeapon_Move`
  (params (CanMove :type Boolean))
  (returns (Result :type Boolean))
  (return false))

(fn `SetWeapon_State`
  (params (State :type "/Game/Enum/E_PlayerState Enum" :default "NewEnumerator0"))
  (returns (Result :type "/Game/Enum/E_PlayerState Enum"))
  (return "NewEnumerator0"))

(fn `SetWeapon_Type`
  (params (WeaponType :type "/Game/안지워지는쓰레기/E_WeaponType Enum" :default "NewEnumerator2"))
  (returns (Result :type "/Game/안지워지는쓰레기/E_WeaponType Enum"))
  (return "NewEnumerator2"))

(fn `Weapon_Change`
  (params (`New Weapon` :type "/Game/Items/BP_Items Object Reference"))
  (returns (Weapon :type "/Game/Items/BP_Items Object Reference"))
  (return null))